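; WaterStream is an actor that pushes the player character along a set direction while they are inside its Collision volume.
; Begin and end overlap events toggle a flag for the player character only.
; While the flag is set, Tick launches the controlled pawn additively by PushDirection times PushForce, scaled by delta time.
; The construction script rotates an Arrow component to show the push direction.
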(event `self.ReceiveTick`
  (params (DeltaSeconds :type "Float (single-precision)"))
  (if (`self.IsOverlapping`)
    (bind _asplayer_character (cast `/Game/OriginalContent/Blueprints/PlayerCharacter` (`Controller.K2_GetPawn` (`GameplayStatics.GetPlayerController` 0))))
    (`Character.LaunchCharacter` _asplayer_character (* (* (`self.PushDirection`) (`self.PushForce`)) (`GameplayStatics.GetWorldDeltaSeconds`)) false false)))

(event `self.Collision.OnComponentBeginOverlap`
  (params (OverlappedComponent :type "PrimitiveComponent Object Reference") (OtherActor :type "Actor Object Reference") (OtherComp :type "PrimitiveComponent Object Reference") (OtherBodyIndex :type Integer) (bFromSweep :type Boolean) (SweepResult :type "HitResult Structure (by ref)"))
  (cast `/Game/OriginalContent/Blueprints/PlayerCharacter` OtherActor)
  (set `self.IsOverlapping` true))

(event `self.Collision.OnComponentEndOverlap`
  (params (OverlappedComponent :type "PrimitiveComponent Object Reference") (OtherActor :type "Actor Object Reference") (OtherComp :type "PrimitiveComponent Object Reference") (OtherBodyIndex :type Integer))
  (cast `/Game/OriginalContent/Blueprints/PlayerCharacter` OtherActor)
  (set `self.IsOverlapping` false))

(fn `UserConstructionScript`
  (`SceneComponent.K2_SetRelativeRotation` (`self.Arrow`) (`KismetMathLibrary.Conv_VectorToRotator` (`self.PushDirection`)) false false))