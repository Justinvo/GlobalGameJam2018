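; A moving platform that travels back and forth between two relative positions at a constant speed.
; Tick moves the Platform component with VInterpToConstant toward the current target and switches targets once it arrives.
; When OnlyStartMovingWhenPlayerIsClose is set, it waits at each endpoint until a PlayerCharacter overlaps the Sphere, which drives the PlayerClose flag.
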(event `self.Sphere.OnComponentEndOverlap`
  (params (OverlappedComponent :type "PrimitiveComponent Object Reference") (OtherActor :type "Actor Object Reference") (OtherComp :type "PrimitiveComponent Object Reference") (OtherBodyIndex :type Integer))
  (cast `/Game/OriginalContent/Blueprints/PlayerCharacter` OtherActor)
  (set `self.PlayerClose` false))

(event `self.Sphere.OnComponentBeginOverlap`
  (params (OverlappedComponent :type "PrimitiveComponent Object Reference") (OtherActor :type "Actor Object Reference") (OtherComp :type "PrimitiveComponent Object Reference") (OtherBodyIndex :type Integer) (bFromSweep :type Boolean) (SweepResult :type "HitResult Structure (by ref)"))
  (cast `/Game/OriginalContent/Blueprints/PlayerCharacter` OtherActor)
  (set `self.PlayerClose` true))

(event `self.ReceiveTick`
  (params (DeltaSeconds :type "Float (single-precision)"))
  (bind _platform (`self.Platform`))
  (bind _returnvalue_location (`KismetMathLibrary.BreakTransform` (`SceneComponent.GetRelativeTransform` (`self.Platform`))))
  (bind _returnvalue_location_2 (`KismetMathLibrary.BreakTransform` (`SceneComponent.GetRelativeTransform` (`self.Platform`))))
  (bind _returnvalue_location_3 (`KismetMathLibrary.BreakTransform` (`SceneComponent.GetRelativeTransform` (`self.Platform`))))
  (bind _returnvalue_location_4 (`KismetMathLibrary.BreakTransform` (`SceneComponent.GetRelativeTransform` (`self.Platform`))))
  (switch `int` (`self.PositionMovingTo`)
    (:`1`
      (`SceneComponent.K2_SetRelativeLocation` _platform (`KismetMathLibrary.VInterpTo_Constant` _returnvalue_location_2 (`self.Position01`) (`GameplayStatics.GetWorldDeltaSeconds`) (`self.PlatformSpeed`)) false false)
      (if (== (`self.Position01`) _returnvalue_location_4 :`ErrorTolerance` 0.0)
        (if (`self.OnlyStartMovingWhenPlayerIsClose`)
          (if (`self.PlayerClose`)
            (`KismetSystemLibrary.Delay` 0.0)
            (set `self.PositionMovingTo` 2 :!label _label))
          (else
            (goto _label)))))
    (:`2`
      (`SceneComponent.K2_SetRelativeLocation` _platform (`KismetMathLibrary.VInterpTo_Constant` _returnvalue_location (`self.Position02`) (`GameplayStatics.GetWorldDeltaSeconds`) (`self.PlatformSpeed`)) false false)
      (if (== (`self.Position02`) _returnvalue_location_3 :`ErrorTolerance` 0.0)
        (if (`self.OnlyStartMovingWhenPlayerIsClose`)
          (if (`self.PlayerClose`)
            (`KismetSystemLibrary.Delay` 0.0)
            (set `self.PositionMovingTo` 1 :!label _label_2))
          (else
            (goto _label_2)))))))

(fn `UserConstructionScript`)