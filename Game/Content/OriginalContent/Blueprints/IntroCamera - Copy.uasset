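; An intro camera pawn that takes player control at start, looks at a star, then turns to the player character and hands over possession.
; Tick smoothly rotates the camera toward the current target with RInterpTo.
; After a configurable delay, BeginPlay retargets to the PlayerCharacter and flips a FlipFlop whose output gates an FOV zoom in Tick, then possesses the character four seconds later.
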(event `self.ReceiveTick`
  (params (DeltaSeconds :type "Float (single-precision)"))
  (bind _camera (`self.Camera`))
  (bind _camera_2 (`self.Camera`))
  ;[1 1 1] Interp Camera Rotation to star
  (`SceneComponent.K2_SetWorldRotation` _camera_2 (`KismetMathLibrary.RInterpTo` (`SceneComponent.K2_GetComponentRotation` _camera_2) (`KismetMathLibrary.FindLookAtRotation` (`SceneComponent.K2_GetComponentLocation` (`self.Camera`)) (`SceneComponent.K2_GetComponentLocation` (`Actor.RootComponent` (`self.StarReference`)))) (`GameplayStatics.GetWorldDeltaSeconds`) (`self.CameraLookSpeed`)) false false)
  (if (stale `self.ReceiveBeginPlay` _isa) :!label _label
    (`CameraComponent.SetFieldOfView` _camera (`KismetMathLibrary.FInterpTo` (`CameraComponent.FieldOfView` _camera) 40.0 (`GameplayStatics.GetWorldDeltaSeconds`) 0.5))))

(event `self.ReceiveBeginPlay`
  ;[1 1 1] Find Star
  (`Controller.Possess` (`GameplayStatics.GetPlayerController` 0) self)
  (bind _outactors (`GameplayStatics.GetAllActorsWithTag` "star"))
  (set `self.StarReference` (`|GetArrayItem` _outactors))
  (`KismetSystemLibrary.Delay` (`self.Duration`))
  (bind _outactors_2 (`GameplayStatics.GetAllActorsOfClass` "/Game/OriginalContent/Blueprints/PlayerCharacter.PlayerCharacter_C"))
  (`|ExecutionSequence`
    (:`then_0`
      (bind _isa (`/Engine/EditorBlueprintResources/StandardMacros.FlipFlop`)
        (:`B`
          (goto _label))))
    (:`then_1`
      (bind _output (`|GetArrayItem` _outactors_2))
      (set `self.StarReference` _output)
      (`KismetSystemLibrary.Delay` 4.0)
      (`Controller.Possess` (`GameplayStatics.GetPlayerController` 0) _output))))

(fn `UserConstructionScript`)