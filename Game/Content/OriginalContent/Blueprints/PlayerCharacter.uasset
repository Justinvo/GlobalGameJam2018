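; Player character Blueprint with camera-relative movement, jumping, dashing and an adjustable spring-arm camera.
; CheckMechanic gates abilities on unlock flags, with the highest unlocked jump tier setting JumpMaxCount before jumping.
; Dash launches the character along the camera's forward vector, with a DoOnce that resets on landing.
; Zoom uses the scroll wheel or middle-mouse hold, where the MouseZoom timeline turns vertical mouse movement into clamped arm length while locking pitch.
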(event `self.OnLanded`
  (params (Hit :type "HitResult Structure (by ref)"))
  ;[1 1 1] Dash
  (goto _label :!via `Reset`))

(event `InputAction|Dash`
  (params (Key :type "Key Structure"))
  ;[1 1 1] Dash
  (:`Pressed`
    (`self.CheckMechanic` "NewEnumerator3"
      (:`Unlocked`
        (`/Engine/EditorBlueprintResources/StandardMacros.DoOnce` false :!label _label
          (:`Completed`
            (`self.LaunchCharacter` (* (`SceneComponent.GetForwardVector` (`self.Camera`)) (`self.DashForce`)))))))))

(event `InputAction|Jump`
  (params (Key :type "Key Structure"))
  ;[1 1 1] Jumping
  (:`Pressed`
    (`self.CheckMechanic` "NewEnumerator2"
      (:`Unlocked`
        _)
      (:`Locked`
        (`self.CheckMechanic` "NewEnumerator1"
          (:`Unlocked`
            _)
          (:`Locked`
            (`self.CheckMechanic` "NewEnumerator0"
              (:`Unlocked`
                _))))))
    (`self.Jump`))
  (:`Released`
    (`self.StopJumping`)))

(event `InputAxis|ForwardMovement`
  (params (AxisValue :type "Float (single-precision)"))
  ;[1 1 1] Walking
  (`self.AddMovementInput` (`SceneComponent.GetForwardVector` (`self.Camera`)) AxisValue))

(event `InputAxis|RightMovement`
  (params (AxisValue :type "Float (single-precision)"))
  ;[1 1 1] Walking
  (`self.AddMovementInput` (`SceneComponent.GetRightVector` (`self.Camera`)) AxisValue))

(event `InputAxis|LookUp`
  (params (AxisValue :type "Float (single-precision)"))
  ;[1 1 1] Camera
  ;;[1 1 1] Camera Look up & Turning
  (if (not (`self.CameraLookUpLocked`))
    (`self.AddControllerPitchInput` (* AxisValue -1.0))))

(event `InputAxis|Turn`
  (params (AxisValue :type "Float (single-precision)"))
  ;[1 1 1] Camera
  ;;[1 1 1] Camera Look up & Turning
  (`self.AddControllerYawInput` AxisValue))

(event `InputAxis|CameraZoom`
  (params (AxisValue :type "Float (single-precision)"))
  (bind _springarm (`self.SpringArm`))
  ;[1 1 1] Camera
  ;;[1 1 1] CameraZoom using scroll wheel
  (set `SpringArmComponent.TargetArmLength` (`KismetMathLibrary.FClamp` (+ (* AxisValue (* (`self.CameraZoomSpeed`) -1.0)) (`SpringArmComponent.TargetArmLength` _springarm)) (`self.MinCameraZoom`) (`self.MaxCameraZoom`)) _springarm))

(event `Key|MiddleMouseButton`
  (params (Key :type "Key Structure"))
  (bind _springarm (`self.SpringArm`))
  ;[1 1 1] Camera
  ;;[1 1 1] Maya Controls for Xandra lmfao
  (:`Pressed`
    (`Timeline|MouseZoom` :!via `PlayFromStart` :!label _label_2
      (:`Update`
        (set `self.CameraLookUpLocked` true)
        (set `SpringArmComponent.TargetArmLength` (`KismetMathLibrary.FClamp` (+ (* (* (`self.GetInputAxisValue`) -1.0) (`self.CameraZoomSpeed`)) (`SpringArmComponent.TargetArmLength` _springarm)) (`self.MinCameraZoom`) (`self.MaxCameraZoom`)) _springarm))))
  (:`Released`
    (set `self.CameraLookUpLocked` false)
    (goto _label_2 :!via `Stop`)))

(fn `UserConstructionScript`)